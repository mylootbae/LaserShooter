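; BP_LaserShowable is an actor that stays hidden and non-collidable until a laser target is hit, then appears.
; On BeginPlay it hides its Cube, disables actor collision and binds Show to the Target's OnTargetHit event, printing a warning if Target is invalid.
; Show fires once, unbinding all listeners from that event, including other actors', then making the cube visible and re-enabling collision.
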(event `self.ReceiveBeginPlay`
  (`SceneComponent.SetVisibility` (`self.Cube`) false false)
  (`self.SetActorEnableCollision` false)
  (bind _target (`self.Target`)
    (:`then`
      (add `/Game/Lasery/Target/BP_Target.OnTargetHit` _target (delegate `Show`)))
    (:`else`
      (`KismetSystemLibrary.PrintString` "Target is not Valid!!!" true true (struct :`R` 1.0 :`G` 0.046926 :`A` 1.0)))))

(event `Show`
  (clear `/Game/Lasery/Target/BP_Target.OnTargetHit` (`self.Target`))
  (`SceneComponent.SetVisibility` (`self.Cube`) true false)
  (`self.SetActorEnableCollision` true))

(fn `UserConstructionScript`)